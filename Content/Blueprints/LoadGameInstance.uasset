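; LoadGameInstance is a helper, named as a game instance, for showing loading screens and starting play.
; Three separate functions each create a different widget for player controller 0 and add it to the viewport: WB_Loading, WB_Loading2 and NewWidgetBlueprint2.
; Play opens the level NewMap by name and does not itself show or remove any of these screens.
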(fn `play`
  (`GameplayStatics.OpenLevel` "NewMap"))

(fn `ShowLoadingScreen`
  (bind _returnvalue (`|CreateWidget` "/Game/Blueprints/WB_Loading.WB_Loading_C" (`GameplayStatics.GetPlayerController` 0)))
  (`UserWidget.AddToViewport` _returnvalue 0))

(fn `ShowLoadingScreen2`
  (bind _returnvalue (`|CreateWidget` "/Game/Blueprints/WB_Loading2.WB_Loading2_C" (`GameplayStatics.GetPlayerController` 0)))
  (`UserWidget.AddToViewport` _returnvalue 0))

(fn `ShowLoadingScreen3`
  (bind _returnvalue (`|CreateWidget` "/Game/Blueprints/NewWidgetBlueprint2.NewWidgetBlueprint2_C" (`GameplayStatics.GetPlayerController` 0)))
  (`UserWidget.AddToViewport` _returnvalue 0))